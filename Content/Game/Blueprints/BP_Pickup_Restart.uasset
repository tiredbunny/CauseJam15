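; BP_Pickup_Restart is a pickup that sends the player back to a randomly chosen PlayerStart.
; BeginPlay caches every PlayerStart actor in the level.
; Any actor overlap moves player 0's pawn to a random cached start with a swept teleport, without checking what overlapped, then destroys the pickup.
; Only location is set; the pawn's rotation and other state are untouched.
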(event `self.ReceiveBeginPlay`
  (`parent.ReceiveBeginPlay`)
  (bind _outactors (`GameplayStatics.GetAllActorsOfClass` "/Script/Engine.PlayerStart"))
  (set `self.PlayerStarts` _outactors))

(event `self.ReceiveTick`
  (params (DeltaSeconds :type "Float (single-precision)"))
  (`parent.ReceiveTick` DeltaSeconds))

(event `self.ReceiveActorBeginOverlap`
  (params (OtherActor :type "Actor Object Reference"))
  (bind _playerstarts (`self.PlayerStarts`))
  (`self.K2_SetActorLocation` (`GameplayStatics.GetPlayerPawn` 0) (`self.K2_GetActorLocation` (`|GetArrayItem` _playerstarts (`KismetMathLibrary.RandomIntegerInRange` 0 (- (`KismetArrayLibrary.Array_Length` _playerstarts) 1)))) true true)
  (`self.K2_DestroyActor`))

(fn `UserConstructionScript`
  (`parent.UserConstructionScript`))