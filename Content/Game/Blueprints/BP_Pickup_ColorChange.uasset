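; BP_Pickup_ColorChange is a pickup that gives the player's ball character a random new look.
; On any actor overlap it casts player pawn 0 to BP_Character, without checking which actor overlapped.
; A random integer selects one of five materials (chrome, metals or lake water) for the character's Sphere component.
; The pickup then destroys itself.
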(event `self.ReceiveBeginPlay`
  (`parent.ReceiveBeginPlay`))

(event `self.ReceiveTick`
  (params (DeltaSeconds :type "Float (single-precision)"))
  (`parent.ReceiveTick` DeltaSeconds))

(event `self.ReceiveActorBeginOverlap`
  (params (OtherActor :type "Actor Object Reference"))
  (bind _asbp_character (cast `/Game/Game/Player/BP_Character` (`GameplayStatics.GetPlayerPawn` 0)))
  (switch `int` (`KismetMathLibrary.RandomIntegerInRange` 0 4)
    (:`0`
      (bind _sphere (`/Game/Game/Player/BP_Character.Sphere` _asbp_character))
      (`PrimitiveComponent.SetMaterial` _sphere 0 "/Engine/EditorMeshes/ColorCalibrator/M_ChromeBall.M_ChromeBall"))
    (:`1`
      (`PrimitiveComponent.SetMaterial` _sphere 0 "/Game/StarterContent/Materials/M_Metal_Gold.M_Metal_Gold"))
    (:`2`
      (`PrimitiveComponent.SetMaterial` _sphere 0 "/Game/StarterContent/Materials/M_Metal_Burnished_Steel.M_Metal_Burnished_Steel"))
    (:`3`
      (`PrimitiveComponent.SetMaterial` _sphere 0 "/Game/StarterContent/Materials/M_Metal_Copper.M_Metal_Copper"))
    (:`4`
      (`PrimitiveComponent.SetMaterial` _sphere 0 "/Game/StarterContent/Materials/M_Water_Lake.M_Water_Lake")))
  (`self.K2_DestroyActor`))

(fn `UserConstructionScript`
  (`parent.UserConstructionScript`))