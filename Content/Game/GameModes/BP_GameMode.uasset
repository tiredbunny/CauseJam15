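; BP_GameMode runs a countdown game mode that ends in "Game Over" when time runs out.
; BeginPlay sets game-only input, creates the WB_GameUI widget and starts a fast looping timer that decrements Time and updates its on-screen text.
; ShowEndScreen, guarded by DoOnce, pauses the timer, displays the result text, Play Again button and background blur, then switches to UI-only input with a visible cursor.
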(event `self.ReceiveBeginPlay`
  (`WidgetBlueprintLibrary.SetInputMode_GameOnly` (`GameplayStatics.GetPlayerController` 0) true)
  (bind _returnvalue (`|CreateWidget` "/Game/Game/UI/WB_GameUI.WB_GameUI_C"))
  (bind _output_get (set `self.WidgetGameUIRef` _returnvalue))
  (`UserWidget.AddToViewport` _output_get 0)
  (bind _returnvalue_2 (`KismetSystemLibrary.K2_SetTimerDelegate` (delegate `EventTimer`) 0.01 true))
  (set `self.Timer` _returnvalue_2))

(event `EventTimer`
  (bind _result (`/Engine/EditorBlueprintResources/StandardMacros.DecrementInt` (`self.Time`))
    (:`  `
      (bind _output_get (set `self.Time` _result))
      (`TextBlock.SetText` (`/Game/Game/UI/WB_GameUI.TextTimer` (`self.WidgetGameUIRef`)) (`KismetTextLibrary.Conv_IntToText` _output_get))
      (if (<= _output_get 0)
        (`self.ShowEndScreen` "Game Over")))))

(event `ShowEndScreen`
  (params (ResultText :type Text))
  (bind _returnvalue (`GameplayStatics.GetPlayerController` 0))
  (bind _widgetgameuiref (`self.WidgetGameUIRef`))
  (`/Engine/EditorBlueprintResources/StandardMacros.DoOnce` false
    (:`Completed`
      (`KismetSystemLibrary.K2_PauseTimerHandle` (`self.Timer`))
      (`TextBlock.SetText` (`/Game/Game/UI/WB_GameUI.TextStatus` _widgetgameuiref) ResultText)
      (`Widget.SetVisibility` (`/Game/Game/UI/WB_GameUI.ButtonPlayAgain` _widgetgameuiref) "Visible")
      (`Widget.SetVisibility` (`/Game/Game/UI/WB_GameUI.BackgroundBlur` _widgetgameuiref) "SelfHitTestInvisible")
      (`WidgetBlueprintLibrary.SetInputMode_UIOnlyEx` _returnvalue null "DoNotLock" true)
      (set `PlayerController.bShowMouseCursor` true _returnvalue))))

(fn `UserConstructionScript`)