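; Player Blueprint with a sphere body that tells the player controller whether jumping is allowed.
; Every tick it traces from the sphere's center to just below its bottom and sets CanJump on BP_PlayerController, true only when the hit actor is tagged "Ground".
; An alternative hit-based ground check is left disconnected from the sphere's hit event and never runs.
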(event `self.ReceiveTick`
  (params (DeltaSeconds :type "Float (single-precision)"))
  (bind (_origin _boxextent _sphereradius) (`KismetSystemLibrary.GetComponentBounds` (`self.Sphere`)))
  ;[1 1 1] Checking CanJump
  (bind (_outhit _returnvalue) (`KismetSystemLibrary.LineTraceSingleForObjects` (`KismetMathLibrary.MakeVector` (.x _origin) (.y _origin) (.z _origin)) (`KismetMathLibrary.MakeVector` (.x _origin) (.y _origin) (- (- (.z _origin) _sphereradius) 0.1)) (`self.JumpObjects`)))
  (bind _asbp_player_controller (cast `/Game/Game/Player/BP_PlayerController` (`GameplayStatics.GetPlayerController` 0)))
  (if _returnvalue
    (if (`self.ActorHasTag` (`.HitActor` (`GameplayStatics.BreakHitResult` _outhit)) "Ground")
      (set `/Game/Game/Player/BP_PlayerController.CanJump` true _asbp_player_controller)
      (else
        (set `/Game/Game/Player/BP_PlayerController.CanJump` false _asbp_player_controller :!label _label)))
    (else
      (goto _label))))

(event `self.Sphere.OnComponentHit`
  (params (HitComponent :type "PrimitiveComponent Object Reference") (OtherActor :type "Actor Object Reference") (OtherComp :type "PrimitiveComponent Object Reference") (NormalImpulse :type "Vector Structure") (Hit :type "HitResult Structure (by ref)"))
  ;[1 1 1] On Hit Ground (Disabled)
)

(fn `UserConstructionScript`)